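; Base character Blueprint providing interaction, weapon handling, aim and shoulder-swap state, and debug printouts of health changes.
; Use targets a BI_Interaction actor found by a camera sphere trace, falling back to InteractSphere overlaps.
; Weapon switching reads DT_WeaponStats, destroys the old weapon, then spawns and attaches a class chosen by weapon type, with fire and reload forwarded as messages.
; Character configuration and muzzle-rotation functions are empty stubs.
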(event `self.ReceiveTick`
  (params (DeltaSeconds :type "Float (single-precision)"))
  (`self.UpdateWeaponMuzzleRotation`))

(event `self.ReceiveBeginPlay`
  (`self.ConfigureCharacter`))

(event `self.InteractSphere.OnComponentBeginOverlap`
  (params (OverlappedComponent :type "PrimitiveComponent Object Reference") (OtherActor :type "Actor Object Reference") (OtherComp :type "PrimitiveComponent Object Reference") (OtherBodyIndex :type Integer) (bFromSweep :type Boolean) (SweepResult :type "HitResult Structure (by ref)"))
  ; Overlap logic for actor to interact
)

(event `self.InteractSphere.OnComponentEndOverlap`
  (params (OverlappedComponent :type "PrimitiveComponent Object Reference") (OtherActor :type "Actor Object Reference") (OtherComp :type "PrimitiveComponent Object Reference") (OtherBodyIndex :type Integer))
  ; Overlap logic for actor to interact
)

(event `self.AC_Health.OnHealthUpdated`
  (params (CurrentHP :type Integer) (IsDead :type Boolean) (IsItDamage :type Boolean))
  (if (not IsDead)
    (`KismetSystemLibrary.PrintString` (`KismetStringLibrary.Concat_StrStr` (`KismetStringLibrary.Conv_IntToString` CurrentHP) "/" (`KismetStringLibrary.Conv_IntToString` (`/Game/Blueprints/Components/AC_Health.MaxHP` (`self.AC_Health`))) " " (`KismetSystemLibrary.GetDisplayName` self)) true true (`KismetMathLibrary.SelectColor` (struct :`R` 0.192708 :`G` 0.007107 :`B` 0.009867 :`A` 1.0) (struct :`R` 0.1875 :`G` 0.932981 :`B` 1.0 :`A` 1.0) IsItDamage) 5.0 "Health")
    (else
      (`KismetSystemLibrary.PrintString` (`KismetStringLibrary.Concat_StrStr` (`KismetSystemLibrary.GetDisplayName` self) " - DIED") true true (struct :`A` 1.0)))))

(fn `ActionAim`
  (params (IsPressed :type Boolean))
  (set `self.IsInAim` IsPressed))

(fn `ActionMain`
  (params (IsPressed :type Boolean))
  (message `/Game/Blueprints/GameEntities/BI_Shooting.InitShootingProcess` (`self.CurrentWeaponActor`) (`local.IsPressed`)))

(fn `ActionReload`
  (message `/Game/Blueprints/GameEntities/BI_Shooting.InitReloadingProcess` (`self.CurrentWeaponActor`)))

(fn `ActionUse`
  (bind (_successful _outactor) (`self.GetFirstOverlappedActorWithInterface`))
  (if _successful
    (set `self.ActorToInteract` _outactor)
    ; Interaction with active objects
    (bind _actortointeract (`self.ActorToInteract`)
      (:`then`
        (bind _succes (message `/Game/Blueprints/GameEntities/BI_Interaction.Interact` _actortointeract self))
        (if _succes
          (`KismetSystemLibrary.PrintString` "Successfuly use" true true (struct :`G` 0.66 :`B` 1.0 :`A` 1.0) 5.0)))
      (:`else`))))

(fn `ConfigureCharacter`)

(fn `GetCurrentCharName`
  (returns (Success :type Boolean) (CurrentCharName :type Name))
  (if (!= (`self.CurrentCharName`) "None")
    (return true (`self.CurrentCharName`))
    (else
      (`KismetSystemLibrary.PrintString` "Configure Failed" false)
      (return false (`self.CurrentCharName`)))))

(fn `GetFirstOverlappedActorWithInterface`
  (returns (Successful :type Boolean) (OutActor :type "Actor Object Reference"))
  (locals (L_HitActor :type "Actor Object Reference"))
  (bind _returnvalue (`self.GetComponentByClass` self "/Script/Engine.CameraComponent"))
  (bind _returnvalue_2 (`SceneComponent.K2_GetComponentLocation` _returnvalue))
  (`|ExecutionSequence`
    (:`then_0`
      (`/Engine/EditorBlueprintResources/StandardMacros.IsValid` _returnvalue
        (:`Is Valid`
          (bind (_outhit _returnvalue_3) (`KismetSystemLibrary.SphereTraceSingle` :`Start` _returnvalue_2 :`End` (+ _returnvalue_2 (* (`SceneComponent.GetForwardVector` _returnvalue) 500.0)) :`Radius` 25.0 :`TraceChannel` "TraceTypeQuery3" :`bTraceComplex` true :`DrawTime` 1.0))
          (if _returnvalue_3
            (bind _output_get (set `local.L_HitActor` (`.HitActor` (`GameplayStatics.BreakHitResult` _outhit))))
            (if (`KismetSystemLibrary.DoesImplementInterface` _output_get "/Game/Blueprints/GameEntities/BI_Interaction.BI_Interaction_C")
              (`self.ActorToInteract`
                (:`then`
                  (if (== (`local.L_HitActor`) (`self.ActorToInteract`))
                    (return true (`self.ActorToInteract`))
                    (else
                      _)))
                (:`else`
                  _))
              (return true (`local.L_HitActor`)))))))
    (:`then_1`
      (for _array_element (`PrimitiveComponent.GetOverlappingActors` (`self.InteractSphere`) "/Script/Engine.Actor")
        (set `local.L_HitActor` _array_element)
        (if (`KismetSystemLibrary.DoesImplementInterface` (`local.L_HitActor`) "/Game/Blueprints/GameEntities/BI_Interaction.BI_Interaction_C")
          (return true (`local.L_HitActor`))))
      (return false null))))

(fn `GetMainStatsStruct`
  (returns (Success :type Boolean) (MainStats :type "/Game/Blueprints/Structures/STRUCT_MainStats Structure"))
  (bind (_success _mainstats) (`/Game/Blueprints/GameEntities/BFL_TPAA.GetMainStatsStructByName` (`self.CurrentCharName`)))
  (return _success _mainstats))

(fn `SpawnWeapon`
  (params (InWeaponName :type Name) (InWeaponType :type "/Game/Blueprints/Enums/ENUM_WeaponType Enum" :default "NewEnumerator0"))
  (if (!= (`local.InWeaponName`) "None")
    (if (not (`KismetSystemLibrary.IsValid` (`self.CurrentWeaponActor`)))
      (bind _returnvalue (`|SpawnActorFromClass` (select `/Game/Blueprints/Enums/ENUM_WeaponType` (`local.InWeaponType`) :`NewEnumerator0` "/Game/Blueprints/Weapon/BP_Weapon_Pistol_A.BP_Weapon_Pistol_A_C" :`NewEnumerator1` "/Game/Blueprints/Weapon/BP_Weapon_Rifle_A.BP_Weapon_Rifle_A_C" :`NewEnumerator2` "/Game/Blueprints/Weapon/BP_Weapon_Shotgun_A.BP_Weapon_Shotgun_A_C" :`NewEnumerator3` "/Game/Blueprints/Weapon/BP_WeaponGrenadeLauncher_A.BP_WeaponGrenadeLauncher_A_C" :`NewEnumerator4` "/Game/Blueprints/Weapon/BP_WeaponSniperRifle_A.BP_WeaponSniperRifle_A_C" :!type "Actor Class Reference") (`SceneComponent.K2_GetComponentToWorld` (`self.WeaponScene`)) "Undefined" "MultiplyWithRoot" self null))
      (set `self.CurrentWeaponActor` _returnvalue)
      (`self.K2_AttachToComponent` (`self.CurrentWeaponActor`) (`self.WeaponScene`) "None" "SnapToTarget" "SnapToTarget" "KeepRelative" true)
      (message `/Game/Blueprints/GameEntities/BI_Shooting.InitWeaponConfigure` (`self.CurrentWeaponActor`) (`local.InWeaponName`))
      (set `self.CurrentWeaponName` (`local.InWeaponName`)))))

(fn `SwitchAim`
  (set `self.IsInAim` (not (`self.IsInAim`))))

(fn `SwitchShoulder`
  (set `self.bIsCameraAtRightShoulder` (not (`self.bIsCameraAtRightShoulder`))))

(fn `UpdateCurrentWeapon`
  (params (InWeaponName :type Name))
  (locals (L_Name :type Name :default "None") (L_Stats :type "/Game/Blueprints/Structures/STRUCT_WeaponStats Structure"))
  (`|ExecutionSequence`
    (:`then_0`
      (if (!= (`local.InWeaponName`) "None")
        (set `local.L_Name` (`local.InWeaponName`))
        (elif (`BlueprintMapLibrary.Map_IsNotEmpty` (`/Game/Blueprints/Components/AC_Backpack.AwalableWeapon` (`self.AC_Backpack`)))
          (bind _keys (`BlueprintMapLibrary.Map_Keys` (`/Game/Blueprints/Components/AC_Backpack.AwalableWeapon` (`self.AC_Backpack`))))
          (set `local.L_Name` (`|GetArrayItem` _keys)))))
    (:`then_1`
      (bind _returnvalue (`|GetDataTableRow` "/Game/Blueprints/DataTables/DT_WeaponStats.DT_WeaponStats" (`local.L_Name`))
        (:`then`
          (set `local.L_Stats` _returnvalue)
          (`|ExecutionSequence`
            (:`then_0`
              (bind _currentweaponactor (`self.CurrentWeaponActor`)
                (:`then`
                  (message `/Game/Blueprints/GameEntities/BI_Shooting.InitWeaponActivation` _currentweaponactor false)
                  ;[1 0 0.05551] FIX ME
                  (`self.K2_DestroyActor` (`self.CurrentWeaponActor`))
                  (set `self.CurrentWeaponActor` null)
                  (set `self.CurrentWeaponMuzzle` null))
                (:`else`)))
            (:`then_1`
              (`self.SpawnWeapon` (`local.L_Name`) (`.WeaponType_2_BAA875C24868E2297C177092D08B6A91` (break `/Game/Blueprints/Structures/STRUCT_WeaponStats` (`local.L_Stats`)))))))))))

(fn `UpdateWeaponMuzzleRotation`)

(fn `UserConstructionScript`)