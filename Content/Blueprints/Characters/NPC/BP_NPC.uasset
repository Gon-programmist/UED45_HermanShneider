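; BP_NPC is a character Blueprint for NPCs with a health bar widget and a persistent death state.
; BeginPlay binds the health bar to the character.
; When AC_Health reports death, it runs once: records the NPC's index in the save game, disables capsule collision, ragdolls the mesh, hides the bar and starts a timer, apparently for delayed destruction.
; ConfigureCharacter destroys NPCs already saved as killed.
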(event `self.ReceiveBeginPlay`
  (`parent.ReceiveBeginPlay`)
  (bind _aswbp_health_bar (cast `/Game/UI/Widgets/WBP_HealthBar` (`WidgetComponent.GetUserWidgetObject` (`self.WidgetHP`))))
  (`/Game/UI/Widgets/WBP_HealthBar.UpdateCurrentCharacterForHP` _aswbp_health_bar self))

(event `self.AC_Health.OnDied`
  (`/Engine/EditorBlueprintResources/StandardMacros.DoOnce` false
    (:`Completed`
      (`|ExecutionSequence`
        (:`then_0`
          (`self.SetActorTickEnabled` false)
          (bind _outsavegameobj (`/Game/Blueprints/GameEntities/BML_TPAA.SimpleSaveGameCheck`)
            (:`IsValid`
              (`KismetArrayLibrary.Array_AddUnique` (`/Game/Blueprints/Objects/BP_SaveGameObject.KilledNPCs` _outsavegameobj) (`/Game/Blueprints/GameEntities/BFL_TPAA.GetObjectIndexForSaveData` self)))))
        (:`then_1`
          (`PrimitiveComponent.SetCollisionEnabled` (`self.CapsuleComponent`) "NoCollision")
          (`CharacterMovementComponent.SetMovementMode` (`self.CharacterMovement`) "MOVE_Flying" 0))
        (:`then_2`
          (`PrimitiveComponent.SetCollisionProfileName` (`self.Mesh`) "Ragdoll" true)
          (`PrimitiveComponent.SetSimulatePhysics` (`self.Mesh`) true))
        (:`then_3`
          (`SceneComponent.SetVisibility` (`self.WidgetHP`) false false))
        (:`then_4`
          (`KismetSystemLibrary.K2_SetTimerDelegate` (`|CreateDelegate` :!event `OnDeathDelay`) 10.0))))))

(fn `ConfigureCharacter`
  (`parent.ConfigureCharacter`)
  (bind _outsavegameobj (`/Game/Blueprints/GameEntities/BML_TPAA.SimpleSaveGameCheck`)
    (:`IsValid`
      (if (!= (`KismetArrayLibrary.Array_Find` (`/Game/Blueprints/Objects/BP_SaveGameObject.KilledNPCs` _outsavegameobj) (`/Game/Blueprints/GameEntities/BFL_TPAA.GetObjectIndexForSaveData` self)) -1)
        (`self.OnDeathDelay`)))))

(fn `OnDeathDelay`
  (`|ExecutionSequence`
    (:`then_1`
      (`self.K2_DestroyActor`))))

(fn `UserConstructionScript`
  (`parent.UserConstructionScript`))