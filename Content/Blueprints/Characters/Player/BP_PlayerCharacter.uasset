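; Player character Blueprint with a third-person over-the-shoulder camera, weapon aiming and ragdoll death.
; Tick eases spring arm length, shoulder-side socket offset and field of view toward aim or default values.
; A sphere trace from the camera turns the weapon muzzle toward the aimed point, or along the view direction on a miss.
; A looping timer reports noise events; death ragdolls the mesh while the camera slowly rotates to follow it.
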(event `self.ReceiveBeginPlay`
  (`parent.ReceiveBeginPlay`)
  (`KismetSystemLibrary.K2_SetTimerDelegate` (delegate `NoiseEvent`) 0.5 true))

(event `NoiseEvent`
  (`AISense_Hearing.ReportNoiseEvent` (`self.K2_GetActorLocation`) 1.0 self 0.0 "Noise"))

(event `self.AC_Health.OnDied`
  (`PrimitiveComponent.SetCollisionProfileName` (`self.Mesh`) "Ragdoll" true)
  (`PrimitiveComponent.SetSimulatePhysics` (`self.Mesh`) true)
  (set `self.DeathCamera` true))

(event `self.ReceiveTick`
  (params (DeltaSeconds :type "Float (single-precision)"))
  (`parent.ReceiveTick` DeltaSeconds)
  (`self.UpdateCameraParams`)
  ; Death Camera
  (if (`self.DeathCamera`)
    (`SceneComponent.K2_SetWorldRotation` (`self.Camera`) (`KismetMathLibrary.RInterpTo` (`SceneComponent.K2_GetComponentRotation` (`self.Camera`)) (`KismetMathLibrary.FindLookAtRotation` (`SceneComponent.K2_GetComponentLocation` (`self.Camera`)) (`SceneComponent.K2_GetComponentLocation` (`self.Mesh`))) (`GameplayStatics.GetWorldDeltaSeconds`) 1.0) false false)))

(fn `CameraSocketOffsetCalc`
  (returns (OutSocketOffset :type "Vector Structure"))
  (locals (L_YAxis :type "Float (double-precision)"))
  (`|ExecutionSequence`
    (:`then_0`
      (set `local.L_YAxis` (* (`KismetMathLibrary.SelectFloat` (.y (`self.CameraSocketOffsetVectorMin`)) (.y (`self.CameraSocketOffsetVectorMax`)) (`self.IsInAim`)) (`KismetMathLibrary.SelectFloat` 1.0 -1.0 (`self.bIsCameraAtRightShoulder`)))))
    (:`then_1`
      (return (`KismetMathLibrary.MakeVector` (`KismetMathLibrary.SelectFloat` (.x (`self.CameraSocketOffsetVectorMin`)) (.x (`self.CameraSocketOffsetVectorMax`)) (`self.IsInAim`)) (`local.L_YAxis`) (`KismetMathLibrary.SelectFloat` (.z (`self.CameraSocketOffsetVectorMin`)) (.z (`self.CameraSocketOffsetVectorMax`)) (`self.IsInAim`)))))))

(fn `CheckAimingLine`
  (returns (OutWorldRotator :type "Rotator Structure") (IsLineAvailable :type Boolean))
  (locals (L_Distance :type "Float (single-precision)" :default 0.0) (L_Location :type "Vector Structure" :default (0.0 0.0 0.0)))
  (bind _returnvalue (`SceneComponent.K2_GetComponentLocation` (`self.Camera`)))
  (bind _returnvalue_2 (`SceneComponent.K2_GetComponentLocation` (`self.Camera`)))
  (bind (_outhit _returnvalue_3) (`KismetSystemLibrary.SphereTraceSingle` _returnvalue_2 (+ _returnvalue_2 (* (`SceneComponent.GetForwardVector` (`self.Camera`)) 10000.0)) 8.0 "TraceTypeQuery2" true (`|MakeArray` self (`self.CurrentWeaponActor`) :!type "Actor Object Reference")))
  (if _returnvalue_3
    (bind (_bblockinghit _binitialoverlap _time _distance _location) (`GameplayStatics.BreakHitResult` _outhit))
    (set `local.L_Distance` _distance)
    (set `local.L_Location` _location)
    (return (`KismetMathLibrary.FindLookAtRotation` (`SceneComponent.K2_GetComponentLocation` (`self.CurrentWeaponMuzzle`)) (`local.L_Location`)) true)
    (else
      (return (`KismetMathLibrary.FindLookAtRotation` _returnvalue (+ _returnvalue (* (`SceneComponent.GetForwardVector` (`self.Camera`)) 10000.0))) true))))

(fn `UpdateCameraParams`
  (locals (L_TargetArmLength :type "Float (double-precision)" :default 0.0))
  (`|ExecutionSequence`
    (:`then_0`
      (set `local.L_TargetArmLength` (`KismetMathLibrary.SelectFloat` (`self.TargetArmLengthMin`) (`self.TargetArmLengthMax`) (`self.IsInAim`))))
    (:`then_1`
      (set `SpringArmComponent.TargetArmLength` (`KismetMathLibrary.FInterpTo` (`SpringArmComponent.TargetArmLength` (`self.SpringArm`)) (`local.L_TargetArmLength`) (`GameplayStatics.GetWorldDeltaSeconds`) (`self.CameraUpdateInterpSpeed`)) (`self.SpringArm`)))
    (:`then_2`
      (set `SpringArmComponent.SocketOffset` (`KismetMathLibrary.VInterpTo` (`SpringArmComponent.SocketOffset` (`self.SpringArm`)) (`self.CameraSocketOffsetCalc`) (`GameplayStatics.GetWorldDeltaSeconds`) (`self.CameraUpdateInterpSpeed`)) (`self.SpringArm`)))
    (:`then_3`
      (`CameraComponent.SetFieldOfView` (`self.Camera`) (`KismetMathLibrary.FInterpTo` (`CameraComponent.FieldOfView` (`self.Camera`)) (`KismetMathLibrary.SelectFloat` (`self.CameraFieldOfViewMin`) (`self.CameraFieldOfViewMax`) (`self.IsInAim`)) (`GameplayStatics.GetWorldDeltaSeconds`) (`self.CameraUpdateInterpSpeed`))))))

(fn `UpdateWeaponMuzzleRotation`
  (locals (L_Rotator :type "Rotator Structure" :default (struct)))
  (`parent.UpdateWeaponMuzzleRotation`)
  (`self.CurrentWeaponActor`
    (:`then`
      (`self.CurrentWeaponMuzzle`
        (:`then`
          (bind _outweaponstate (message `/Game/Blueprints/GameEntities/BI_Shooting.GetWeaponState` (`self.CurrentWeaponActor`)))
          (switch `/Game/Blueprints/Enums/ENUM_WeaponState` _outweaponstate
            (:`NewEnumerator0`
              _)
            (:`NewEnumerator1`
              _)
            (:`NewEnumerator5`
              _))
          (bind (_outworldrotator _islineavailable) (`self.CheckAimingLine`))
          (set `local.L_Rotator` _outworldrotator)
          (if _islineavailable
            (`SceneComponent.K2_SetWorldRotation` (`self.CurrentWeaponMuzzle`) (`local.L_Rotator`) false false)
            (else
              (`SceneComponent.K2_SetWorldRotation` :`self` (`self.CurrentWeaponMuzzle`)))))
        (:`else`)))
    (:`else`)))

(fn `UserConstructionScript`
  (`parent.UserConstructionScript`))