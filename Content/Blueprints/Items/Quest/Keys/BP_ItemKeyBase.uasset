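; BP_ItemKeyBase is, by name and folder, the base Blueprint for key quest items that go into a backpack.
; Its PutIntoBackpack override finds the AC_Backpack component on ActorOfInteraction and, if valid, adds one quest item under the key's ItemName.
; The parent PutIntoBackpack is never called, so this logic replaces the inherited behavior.
; The event graph holds only disabled stub events.
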(fn `PutIntoBackpack`
  (bind _returnvalue (`self.GetComponentByClass` (`self.ActorOfInteraction`) "/Game/Blueprints/Components/AC_Backpack.AC_Backpack_C"))
  (`/Engine/EditorBlueprintResources/StandardMacros.IsValid` _returnvalue
    (:`Is Valid`
      (`/Game/Blueprints/Components/AC_Backpack.AddQuestItem` _returnvalue (`self.ItemName`) 1))))

(fn `UserConstructionScript`
  (`parent.UserConstructionScript`))