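; Base pickup item that goes into the interacting actor's backpack as a consumable and stays collected through save data.
; Interact, gated by the hint widget's readiness, adds the item name and amount to AC_Backpack, records the item's index in PickedItems, then destroys the actor.
; On BeginPlay, named items already in that list destroy themselves, while unnamed ones print a warning.
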(event `self.ReceiveBeginPlay`
  (`self.ConfigureItem`))

(fn `AfterUseItem`
  (locals (L_Items :type String))
  (`|ExecutionSequence`
    (:`then_0`
      (bind _outsavegameobj (`/Game/Blueprints/GameEntities/BML_TPAA.SimpleSaveGameCheck`)
        (:`IsValid`
          (bind _pickeditems (`/Game/Blueprints/Objects/BP_SaveGameObject.PickedItems` _outsavegameobj))
          (`KismetArrayLibrary.Array_AddUnique` _pickeditems (`/Game/Blueprints/GameEntities/BFL_TPAA.GetObjectIndexForSaveData` self))
          (if (`self.Debug`)
            (for _array_element _pickeditems
              (set `local.L_Items` (`KismetStringLibrary.Concat_StrStr` (`KismetStringLibrary.Conv_NameToString` _array_element) " \n" (`local.L_Items`))))
            (`KismetSystemLibrary.PrintString` (`KismetStringLibrary.Concat_StrStr` "Saved items List:" " \n" (`local.L_Items`)) true true (struct :`R` 0.545724 :`G` 0.201556 :`B` 0.887923 :`A` 1.0) 5.0 "ITEMS")))))
    (:`then_1`
      (`self.K2_DestroyActor`))))

(fn `ConfigureItem`
  (if (!= (`self.ItemName`) "None")
    (bind _outsavegameobj (`/Game/Blueprints/GameEntities/BML_TPAA.SimpleSaveGameCheck`)
      (:`IsValid`
        (if (!= (`KismetArrayLibrary.Array_Find` (`/Game/Blueprints/Objects/BP_SaveGameObject.PickedItems` _outsavegameobj) (`/Game/Blueprints/GameEntities/BFL_TPAA.GetObjectIndexForSaveData` self)) -1)
          (`self.K2_DestroyActor`))))
    (else
      (`KismetSystemLibrary.PrintString` (`KismetStringLibrary.Concat_StrStr` "ItemActor" (`KismetSystemLibrary.GetDisplayName` self) "has no Name!")))))

(fn `Interact`
  (params (InteractActor :type "Actor Object Reference"))
  (returns (Succes :type Boolean))
  (set `self.ActorOfInteraction` InteractActor)
  (if (`/Game/Blueprints/Components/AC_HintWidget.IsReadyToInteract` (`self.AC_HintWidget`))
    (`self.UseItem`)
    (return true)
    (else
      (return false))))

(fn `PutIntoBackpack`
  (bind _returnvalue (`self.GetComponentByClass` (`self.ActorOfInteraction`) "/Game/Blueprints/Components/AC_Backpack.AC_Backpack_C"))
  (`/Engine/EditorBlueprintResources/StandardMacros.IsValid` _returnvalue
    (:`Is Valid`
      (`/Game/Blueprints/Components/AC_Backpack.AddConsumableItem` _returnvalue (`self.ItemName`) (`self.Amount`)))))

(fn `UseItem`
  (`self.PutIntoBackpack`)
  (`self.AfterUseItem`))

(fn `UserConstructionScript`)