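; BP_Item_AmmoBase is the base ammo item, which adds its ammo to the interacting actor's backpack.
; Its PutIntoBackpack override requires a positive Amount and a valid AC_Backpack component on ActorOfInteraction.
; It then increases the ammo count through UpdateAmmoByName, keyed by ItemName, and calls AfterUseItem.
; The override does not run the parent implementation, and the event graph holds only disabled placeholder events.
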(fn `PutIntoBackpack`
  (bind _returnvalue (`self.GetComponentByClass` (`self.ActorOfInteraction`) "/Game/Blueprints/Components/AC_Backpack.AC_Backpack_C"))
  (if (> (`self.Amount`) 0)
    (`/Engine/EditorBlueprintResources/StandardMacros.IsValid` _returnvalue
      (:`Is Valid`
        (`/Game/Blueprints/Components/AC_Backpack.UpdateAmmoByName` _returnvalue (`self.ItemName`) (`self.Amount`) true)
        (`self.AfterUseItem`)))))

(fn `UserConstructionScript`
  (`parent.UserConstructionScript`))