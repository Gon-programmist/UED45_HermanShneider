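; Base weapon pickup item that an interacting actor puts into its backpack.
; On BeginPlay it looks up weapon stats by ItemName and shows the weapon's nickname in the hint widget.
; PutIntoBackpack overrides the parent without calling it: with a positive Amount, it finds the actor's AC_Backpack and either adds the weapon or, if already owned, adds that weapon's max rounds as ammo, then runs AfterUseItem.
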(event `self.ReceiveBeginPlay`
  (bind (_success _outweaponstats) (`/Game/Blueprints/GameEntities/BFL_TPAA.GetWeaponStatsStructByName` (`self.ItemName`)))
  (`parent.ReceiveBeginPlay`)
  (if _success
    (`/Game/Blueprints/Components/AC_HintWidget.UpdateHintText` (`self.AC_HintWidget`) (`|FormatText` "Weapon item \n{Nickname}" (`.Nickname_5_08CEC5EE40564CBE3563D998BF1600B6` (break `/Game/Blueprints/Structures/STRUCT_WeaponStats` _outweaponstats))))))

(fn `PutIntoBackpack`
  (locals (L_Backpack :type "/Game/Blueprints/Components/AC_Backpack Object Reference"))
  (if (> (`self.Amount`) 0)
    (bind _output_get (set `local.L_Backpack` (`self.GetComponentByClass` (`self.ActorOfInteraction`) "/Game/Blueprints/Components/AC_Backpack.AC_Backpack_C")))
    (`/Engine/EditorBlueprintResources/StandardMacros.IsValid` _output_get
      (:`Is Valid`
        (`|ExecutionSequence`
          (:`then_0`
            (if (`/Game/Blueprints/Components/AC_Backpack.CheckWeaponItem` (`local.L_Backpack`) (`self.ItemName`))
              (`/Game/Blueprints/Components/AC_Backpack.UpdateAmmoByName` (`local.L_Backpack`) (`self.ItemName`) (`.OutMaxRounds` (`/Game/Blueprints/Components/AC_Backpack.GetMaxRoundsForWeapon` (`local.L_Backpack`) (`self.ItemName`))) true)
              (else
                (`/Game/Blueprints/Components/AC_Backpack.AddWeaponItem` (`local.L_Backpack`) (`self.ItemName`)))))
          (:`then_1`
            (`self.AfterUseItem`)))))))

(fn `UserConstructionScript`
  (`parent.UserConstructionScript`))