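; Backpack actor component that tracks consumable and quest item counts in two name-keyed maps.
; On BeginPlay it restores both maps from the player-component save game when valid, optionally printing their keys in debug; it never writes the save.
; Add functions accumulate amounts and always print the total, while Check and Remove wrap map lookup and deletion.
; Use functions overwrite the stored count with the passed amount rather than subtracting it.
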(event `self.ReceiveBeginPlay`
  (`self.ConfigureBackpack`))

(fn `AddConsumableItem`
  (params (InItemName :type Name) (InAmount :type Integer :default 1))
  (bind (_value _returnvalue) (`BlueprintMapLibrary.Map_Find` (`self.ConsumableItems`) (`local.InItemName`)))
  (if (!= (`local.InItemName`) "None")
    (`|ExecutionSequence`
      (:`then_0`
        (if _returnvalue
          (`BlueprintMapLibrary.Map_Add` (`self.ConsumableItems`) (`local.InItemName`) (+ _value (`local.InAmount`)))
          (else
            (`BlueprintMapLibrary.Map_Add` (`self.ConsumableItems`) (`local.InItemName`) (`local.InAmount`)))))
      (:`then_1`
        (`KismetSystemLibrary.PrintString` (`KismetStringLibrary.Concat_StrStr` "ConsumableItems:" (`KismetStringLibrary.Conv_NameToString` (`local.InItemName`)) "//" (`KismetStringLibrary.Conv_IntToString` (`BlueprintMapLibrary.Map_Find` (`self.ConsumableItems`) (`local.InItemName`)))) true true (struct :`R` 0.159276 :`G` 0.163956 :`B` 0.416667 :`A` 1.0) 5.0 "Backpack")))))

(fn `AddQuestItem`
  (params (InItemName :type Name) (InAmount :type Integer :default 1))
  (bind (_value _returnvalue) (`BlueprintMapLibrary.Map_Find` (`self.QuestItems`) (`local.InItemName`)))
  (if (!= (`local.InItemName`) "None")
    (`|ExecutionSequence`
      (:`then_0`
        (if _returnvalue
          (`BlueprintMapLibrary.Map_Add` (`self.QuestItems`) (`local.InItemName`) (+ _value (`local.InAmount`)))
          (else
            (`BlueprintMapLibrary.Map_Add` (`self.QuestItems`) (`local.InItemName`) (`local.InAmount`)))))
      (:`then_1`
        (`KismetSystemLibrary.PrintString` (`KismetStringLibrary.Concat_StrStr` "QuestItems:" (`KismetStringLibrary.Conv_NameToString` (`local.InItemName`)) "//" (`KismetStringLibrary.Conv_IntToString` (`BlueprintMapLibrary.Map_Find` (`self.QuestItems`) (`local.InItemName`)))) true true (struct :`R` 0.159276 :`G` 0.163956 :`B` 0.416667 :`A` 1.0) 5.0 "Backpack")))))

(fn `CheckConsumableItem`
  (params (InItemName :type Name))
  (returns (Success :type Boolean) (Amount :type Integer))
  (bind (_value _returnvalue) (`BlueprintMapLibrary.Map_Find` (`self.ConsumableItems`) (`local.InItemName`)))
  (return _returnvalue _value))

(fn `CheckQuestItem`
  (params (InItemName :type Name))
  (returns (Success :type Boolean) (Amount :type Integer))
  (bind (_value _returnvalue) (`BlueprintMapLibrary.Map_Find` (`self.QuestItems`) (`local.InItemName`)))
  (return _returnvalue _value))

(fn `ConfigureBackpack`
  (locals (L_SaveGameObj :type "/Game/Blueprints/Objects/BP_SaveGameObject Object Reference") (L_Items :type String :default "Hello"))
  (bind _outsavegameobj (`/Game/Blueprints/GameEntities/BML_TPAA.CheckSaveGameForPlayerComponents` self)
    (:`IsValid`
      (set `local.L_SaveGameObj` _outsavegameobj)
      (`|ExecutionSequence`
        (:`then_0`
          (set `self.ConsumableItems` (`/Game/Blueprints/Objects/BP_SaveGameObject.SavedConsumableItems` (`local.L_SaveGameObj`))))
        (:`then_1`
          (set `self.QuestItems` (`/Game/Blueprints/Objects/BP_SaveGameObject.SavedQuestItems` (`local.L_SaveGameObj`))))
        (:`then_2`
          (if (`self.Debug`)
            (`|ExecutionSequence`
              (:`then_0`
                (bind _keys (`BlueprintMapLibrary.Map_Keys` (`self.ConsumableItems`)))
                (for _array_element _keys
                  (set `local.L_Items` (`KismetStringLibrary.Concat_StrStr` "Consumable:" (`KismetStringLibrary.Conv_NameToString` _array_element) " \n" (`local.L_Items`)))))
              (:`then_1`
                (bind _keys_2 (`BlueprintMapLibrary.Map_Keys` (`self.QuestItems`)))
                (for _array_element_2 _keys_2
                  (set `local.L_Items` (`KismetStringLibrary.Concat_StrStr` "Quest:" (`KismetStringLibrary.Conv_NameToString` _array_element_2) " \n" (`local.L_Items`)))))
              (:`then_2`
                (`KismetSystemLibrary.PrintString` (`KismetStringLibrary.Concat_StrStr` "BackPack Items: \n" (`local.L_Items`)) true true (struct :`G` 0.66 :`B` 1.0 :`A` 1.0) 5.0 "Backpack")))))))))

(fn `RemoveConsumableItem`
  (params (InItemName :type Name))
  (returns (Success :type Boolean))
  (bind _returnvalue (`BlueprintMapLibrary.Map_Remove` (`self.ConsumableItems`) InItemName))
  (return _returnvalue))

(fn `RemoveQuestItem`
  (params (InItemName :type Name))
  (returns (Success :type Boolean))
  (bind _returnvalue (`BlueprintMapLibrary.Map_Remove` (`self.QuestItems`) InItemName))
  (return _returnvalue))

(fn `UseConsumableItem`
  (params (InItemName :type Name) (InAmount :type Integer :default 1))
  (`BlueprintMapLibrary.Map_Add` (`self.ConsumableItems`) InItemName InAmount))

(fn `UseQuestItem`
  (params (InItemName :type Name) (InAmount :type Integer :default 1))
  (`BlueprintMapLibrary.Map_Add` (`self.QuestItems`) InItemName InAmount))