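; Actor component that sets up its owner's movement speeds and restores the player's saved position on BeginPlay.
; It reads main stats from the owner through a message call, applies max walk speed to CharacterMovement with crouch at half, then fires OnCustomMovement.
; Separately, it checks the save game and teleports the owner to the last saved transform, treating a near-zero location as no save.
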(event `self.ReceiveBeginPlay`
  (`self.ConfigureMovement`))

(fn `CheckPlayersavedTransform`
  (params (InTransform :type "Transform Structure"))
  (returns (IsValid :type Boolean) (OutTransform :type "Transform Structure"))
  (return (!= (.location (`local.InTransform`)) (0.0 0.0 0.0) :`ErrorTolerance` 0.01) (`local.InTransform`)))

(fn `ConfigureMovement`
  (bind _returnvalue (`Actor.GetComponentByClass` (`self.GetOwner`) "/Script/Engine.CharacterMovementComponent"))
  (`|ExecutionSequence`
    (:`then_0`
      (bind (_success _mainstats) (message `/Game/Blueprints/GameEntities/BI_Stats.GetMainStatsStruct` (`self.GetOwner`)))
      (if _success
        (`/Engine/EditorBlueprintResources/StandardMacros.IsValid` _returnvalue
          (:`Is Valid`
            (bind (_type _maxhp _maxarmor _maxwalkspeed) (break `/Game/Blueprints/Structures/STRUCT_MainStats` _mainstats))
            (set `CharacterMovementComponent.MaxWalkSpeed` _maxwalkspeed _returnvalue)
            (set `CharacterMovementComponent.MaxWalkSpeedCrouched` (/ _maxwalkspeed 2.0) _returnvalue)
            (`self.OnCustomMovement`)))))
    (:`then_1`
      (bind _outsavegameobj (`/Game/Blueprints/GameEntities/BML_TPAA.CheckSaveGameForPlayerComponents` self)
        (:`IsValid`
          (bind (_isvalid _outtransform) (`self.CheckPlayersavedTransform` (`/Game/Blueprints/Objects/BP_SaveGameObject.PlayerLastTransform` _outsavegameobj)))
          (if _isvalid
            (`Actor.K2_SetActorTransform` (`self.GetOwner`) _outtransform false true)))))))