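; Health component that tracks its owner's current and max HP, handling damage, healing and death.
; On BeginPlay it binds to the owner's damage event, reads MaxHP from the owner's stats struct, then restores saved player HP or fills to maximum.
; Only BP_DamageType damage is applied, truncated to integers.
; Dispatchers broadcast health updates, non-lethal hits with type and causer, and death.
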(event `self.ReceiveBeginPlay`
  (add `Actor.OnTakeAnyDamage` (`self.GetOwner`) (`|CreateDelegate` :!event `OnTakeAnyDamage`))
  (`self.ConfigureHealth`))

(fn `CheckHealth`
  (returns (OnMaxHP :type Boolean))
  (return (== (`self.CurrentHP`) (`self.MaxHP`))))

(fn `ConfigureHealth`
  (bind (_success _mainstats) (message `/Game/Blueprints/GameEntities/BI_Stats.GetMainStatsStruct` (`self.GetOwner`)))
  (if _success
    (set `self.MaxHP` (`.MaxHP_5_775AB5614045D98218F30BA1809E3447` (break `/Game/Blueprints/Structures/STRUCT_MainStats` _mainstats)))
    (bind _outsavegameobj (`/Game/Blueprints/GameEntities/BML_TPAA.CheckSaveGameForPlayerComponents` self)
      (:`IsValid`
        (set `self.CurrentHP` (`/Game/Blueprints/Objects/BP_SaveGameObject.SavedPlayerHP` _outsavegameobj))
        (`self.OnHealthUpdated` (`self.CurrentHP`) (`self.IsDead`)))
      (:`False`
        (`self.HealUp` true)))))

(fn `HealUp`
  (params (InToMaximum :type Boolean :default false) (InAddHP :type Integer))
  (set `self.CurrentHP` (`KismetMathLibrary.SelectInt` (`self.MaxHP`) (`KismetMathLibrary.Min` (+ (`self.CurrentHP`) (`local.InAddHP`)) (`self.MaxHP`)) (`local.InToMaximum`)))
  (`self.OnHealthUpdated` (`self.CurrentHP`) (`self.IsDead`)))

(fn `OnTakeAnyDamage`
  (params (InDamagedActor :type "Actor Object Reference") (InDamage :type "Float (single-precision)") (InDamageType :type "DamageType Object Reference") (InstigatedBy :type "Controller Object Reference") (InDamageCauser :type "Actor Object Reference"))
  (bind _asbp_damage_type (cast `/Game/Blueprints/Objects/BP_DamageType` (`local.InDamageType`)))
  (`self.ReceiveDamage` (`KismetMathLibrary.FTrunc` (`local.InDamage`)) (`/Game/Blueprints/Objects/BP_DamageType.CurrentDamageType` _asbp_damage_type) (`local.InDamageCauser`)))

(fn `ReceiveDamage`
  (params (InDamage :type Integer) (InDamageType :type "/Game/Blueprints/Enums/ENUM_DamageType Enum" :default "NewEnumerator0") (InDamageCauser :type "Actor Object Reference"))
  (if (not (`self.IsDead`))
    (set `self.CurrentHP` (- (`self.CurrentHP`) (`local.InDamage`)))
    (if (> (`self.CurrentHP`) 0)
      (set `self.IsDead` false)
      (else
        (set `self.CurrentHP` 0)
        (set `self.IsDead` true)))
    (`self.OnHealthUpdated` (`self.CurrentHP`) (`self.IsDead`) true)
    (if (`self.IsDead`)
      (`self.OnDied`)
      (else
        (`self.OnDamageRecieved` (`local.InDamage`) (`local.InDamageType`) (`local.InDamageCauser`))))))