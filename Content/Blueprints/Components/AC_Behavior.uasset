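; Actor component that holds its owner's behavior and faction, initialized from the owner's main stats.
; On BeginPlay it requests the main stats struct from the owner and, if that succeeds, stores the current behavior and faction.
; It then calls OnBehaviorUpdate, passing both values along with the attack, chase and retreat distances from those stats.
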(event `self.ReceiveBeginPlay`
  (`self.ConfigureBehaviorAndFactions`))

(fn `ConfigureBehaviorAndFactions`
  (locals (L_mainStats :type "/Game/Blueprints/Structures/STRUCT_MainStats Structure"))
  (bind ((`Behavior_15_0101E7AE4C7915D38FA02597C8F9D1DF` _behavior) (`Faction_18_A3784FCA4697E24B63EDA3934133A705` _faction) (`AttackStartDistance_24_567C38504F10A1948AEE918766993D91` _attackstartdistance) (`ChaseStartDistance_25_D0DB37424A4AEAE0E873F48DE9001635` _chasestartdistance) (`RetreatStartDistance_26_10ED26834495B7AD52C7679954BA0646` _retreatstartdistance) (`RetreatDistance_27_3F8A622E4992E8DBED5A5CA65616E87F` _retreatdistance)) (break `/Game/Blueprints/Structures/STRUCT_MainStats` (`local.L_mainStats`)))
  (bind (_success _mainstats) (message `/Game/Blueprints/GameEntities/BI_Stats.GetMainStatsStruct` (`self.GetOwner`)))
  (if _success
    (set `local.L_mainStats` _mainstats)
    (`|ExecutionSequence`
      (:`then_0`
        (`self.UpdateBehavior` (`.Behavior_15_0101E7AE4C7915D38FA02597C8F9D1DF` (break `/Game/Blueprints/Structures/STRUCT_MainStats` (`local.L_mainStats`))))
        (`self.UpdateFaction` (`.Faction_18_A3784FCA4697E24B63EDA3934133A705` (break `/Game/Blueprints/Structures/STRUCT_MainStats` (`local.L_mainStats`)))))
      (:`then_1`
        (`self.OnBehaviorUpdate` _behavior _faction _attackstartdistance _chasestartdistance _retreatstartdistance _retreatdistance)))))

(fn `UpdateBehavior`
  (params (InCurrentBehavior :type "/Game/Blueprints/Enums/ENUM_Behavior Enum" :default "NewEnumerator0"))
  (set `self.CurrentBehavior` InCurrentBehavior))

(fn `UpdateFaction`
  (params (InCurrentFaction :type "/Game/Blueprints/Enums/ENUM_Faction Enum" :default "NewEnumerator0"))
  (set `self.CurrentFaction` InCurrentFaction))