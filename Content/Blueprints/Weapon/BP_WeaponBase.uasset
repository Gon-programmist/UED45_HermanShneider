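; Base weapon actor that fires type-specific projectiles with audio and muzzle effects, configured by name from DT_WeaponStats.
; While active, Tick turns held shoot input into shots through a timer-driven weapon state machine, broadcasting state changes.
; Reloading rate-scales the owner's montage to reload time and draws ammo from AC_Backpack unless ammo is infinite.
; Configuration applies the owner's damage multiplier and gives owners other than the player auto-reload and infinite ammo.
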(event `self.ReceiveBeginPlay`)

(event `self.ReceiveTick`
  (params (DeltaSeconds :type "Float (single-precision)"))
  (if (`self.InWeaponActive`)
    (`self.Shooting`)))

(event `/Game/Blueprints/GameEntities/BI_Shooting.InitShootingProcess`
  (params (InProcess :type Boolean))
  (`self.ShootInputRecieved` InProcess))

(event `/Game/Blueprints/GameEntities/BI_Shooting.InitUpdateWeaponState`
  (params (InWeaponState :type "/Game/Blueprints/Enums/ENUM_WeaponState Enum" :default "NewEnumerator0"))
  (`self.UpdateWeaponState` InWeaponState))

(event `/Game/Blueprints/GameEntities/BI_Shooting.InitWeaponConfigure`
  (params (InWeaponName :type Name))
  (`self.ConfigureWeapon` InWeaponName))

(event `/Game/Blueprints/GameEntities/BI_Shooting.InitWeaponActivation`
  (params (InActive :type Boolean))
  (`self.ActivateWeapon` InActive))

(event `/Game/Blueprints/GameEntities/BI_Shooting.InitReloadingProcess`
  (`self.Reload`))

(fn `ActivateWeapon`
  (params (InActivation :type Boolean))
  (locals (L_Skel :type "Array of SkeletalMeshComponent Object Reference"))
  (set `self.InWeaponActive` (`local.InActivation`))
  (bind _output_get (set `local.L_Skel` (`self.K2_GetComponentsByClass` "/Script/Engine.SkeletalMeshComponent")))
  (if (`KismetArrayLibrary.Array_IsNotEmpty` _output_get)
    (for _array_element (`local.L_Skel`)
      (`SceneComponent.SetVisibility` _array_element (`local.InActivation`) true))))

(fn `AfterReloadDelayEnds`
  (`self.UpdateWeaponState` "NewEnumerator0")
  ; Reload Ends Feedback
  (`AudioComponent.Play` (`self.ReloadEndAudio`) 0.0))

(fn `AfterShotDelayEnds`
  (if (`|EnumInequality` (`self.CurrentWeaponState`) "NewEnumerator5")
    (`self.UpdateWeaponState` "NewEnumerator0")))

(fn `ConfigureWeapon`
  (params (InWeaponName :type Name))
  (set `self.WeaponName` InWeaponName)
  (if (!= (`self.WeaponName`) "None")
    (bind _returnvalue (`|GetDataTableRow` "/Game/Blueprints/DataTables/DT_WeaponStats.DT_WeaponStats" (`self.WeaponName`))
      (:`then`
        (set `self.WeaponStats` _returnvalue)
        (`|ExecutionSequence`
          (:`then_0`
            (set `self.CurrentRounds` (`.RoundMax_8_3E092F184B562C4574B110BCF31C5381` (break `/Game/Blueprints/Structures/STRUCT_WeaponStats` (`self.WeaponStats`))))
            (set `self.CurrentDamage` (`.Damage_12_60C9AF87477EC86F70E7D0819E743902` (break `/Game/Blueprints/Structures/STRUCT_WeaponStats` (`self.WeaponStats`)))))
          (:`then_1`
            (set `self.AutoReload` (`.AutoReload_20_E28502DF4DE83E263875BE8A22D19C81` (break `/Game/Blueprints/Structures/STRUCT_WeaponStats` (`self.WeaponStats`))))
            (set `self.InfiniteAmmo` (`.InfiniteAmmo_22_CD9E630E485BCCE61D3D1990A3238E71` (break `/Game/Blueprints/Structures/STRUCT_WeaponStats` (`self.WeaponStats`)))))
          (:`then_2`
            (`/Engine/EditorBlueprintResources/StandardMacros.IsValid` (`self.GetOwner`)
              (:`Is Valid`
                (`|ExecutionSequence`
                  (:`then_0`
                    (bind (_success _mainstats) (message `/Game/Blueprints/GameEntities/BI_Stats.GetMainStatsStruct` (`self.GetOwner`)))
                    (if _success
                      (set `self.CurrentDamage` (`KismetMathLibrary.FTrunc` (* (`self.CurrentDamage`) (`.DamageMult_12_6ED10AC745926BF300CE06BEF815E26D` (break `/Game/Blueprints/Structures/STRUCT_MainStats` _mainstats)))))))
                  (:`then_1`
                    (if (!= (`self.GetOwner`) (`GameplayStatics.GetPlayerPawn` 0))
                      (set `self.AutoReload` true)
                      (set `self.InfiniteAmmo` true)))))))))
      (:`RowNotFound`
        (`KismetSystemLibrary.PrintString` "Configure FAILED with Weapon name not found in DT" false)))
    (else
      (`KismetSystemLibrary.PrintString` "Configure FAILED with Weapon Name" false))))

(fn `GetMuzzleScene`
  (returns (OutMuzzleScene :type "SceneComponent Object Reference"))
  (return (`self.MuzzleScene`)))

(fn `GetWeaponName`
  (returns (OutWeaponName :type Name))
  (return (`self.WeaponName`)))

(fn `GetWeaponState`
  (returns (OutWeaponState :type "/Game/Blueprints/Enums/ENUM_WeaponState Enum"))
  (return (`self.CurrentWeaponState`)))

(fn `GetWeaponStats`
  (returns (OutWeaponStats :type "/Game/Blueprints/Structures/STRUCT_WeaponStats Structure") (OutCurrentRounds :type Integer) (OutCurrentDamage :type Integer) (OutCurrentInfiniteAutoReload :type Boolean) (OutCurrentInfiniteAmmo :type Boolean))
  (return (`self.WeaponStats`) (`self.CurrentRounds`) (`self.CurrentDamage`) (`self.AutoReload`) (`self.InfiniteAmmo`)))

(fn `Reload`
  (locals (L_Character :type "Character Object Reference") (L_AnimLength :type "Float (single-precision)" :default 0.0) (L_ReloadAnimMontage :type "AnimMontage Object Reference") (L_Backpack :type "/Game/Blueprints/Components/AC_Backpack Object Reference"))
  (bind _returnvalue (`self.GetComponentByClass` (`self.GetOwner`) "/Game/Blueprints/Components/AC_Backpack.AC_Backpack_C"))
  (if (and (or (not (`self.ShootInProcess`)) (`|EnumEquality` (`self.CurrentWeaponState`) "NewEnumerator2")) (`|EnumInequality` (`self.CurrentWeaponState`) "NewEnumerator3"))
    (`self.UpdateWeaponState` "NewEnumerator3")
    (`|ExecutionSequence`
      (:`then_0`
        ; Reload Starts Feedback
        (`AudioComponent.Play` (`self.ReloadStartAudio`) 0.0))
      (:`then_1`
        ; Reload Animation
        (bind _ascharacter (cast `Character` (`self.GetOwner`)))
        (set `local.L_Character` _ascharacter)
        (bind _output_get (set `local.L_ReloadAnimMontage` (select `/Game/Blueprints/Enums/ENUM_WeaponType` (`.WeaponType_2_BAA875C24868E2297C177092D08B6A91` (break `/Game/Blueprints/Structures/STRUCT_WeaponStats` (`self.WeaponStats`))) :`NewEnumerator0` "/Game/Art/Animations/Characters/BattleRoyale/Rifle_Hip/AM_Reload_Rifle_Hip_Montage.AM_Reload_Rifle_Hip_Montage" :`NewEnumerator1` "/Game/Art/Animations/Characters/BattleRoyale/Rifle_Hip/AM_Reload_Rifle_Hip_Montage.AM_Reload_Rifle_Hip_Montage" :`NewEnumerator2` "/Game/Art/Animations/Characters/BattleRoyale/Rifle_Hip/AM_Reload_Rifle_Hip_Montage.AM_Reload_Rifle_Hip_Montage" :`NewEnumerator3` "/Game/Art/Animations/Characters/BattleRoyale/Rifle_Hip/AM_Reload_Rifle_Hip_Montage.AM_Reload_Rifle_Hip_Montage" :`NewEnumerator4` "/Game/Art/Animations/Characters/BattleRoyale/Rifle_Hip/AM_Reload_Rifle_Hip_Montage.AM_Reload_Rifle_Hip_Montage" :!type "AnimMontage Object Reference")))
        (bind _returnvalue_2 (`Character.PlayAnimMontage` (`local.L_Character`) _output_get 1.0 "None"))
        (set `local.L_AnimLength` _returnvalue_2)
        (if (> (`local.L_AnimLength`) 0.0)
          (`Character.PlayAnimMontage` (`local.L_Character`) (`local.L_ReloadAnimMontage`) (/ (`local.L_AnimLength`) (`.ReloadTime_17_E12FA9884E84FD8781E987B5FF3FFC03` (break `/Game/Blueprints/Structures/STRUCT_WeaponStats` (`self.WeaponStats`)))) "None")))
      (:`then_2`
        (if (and (`KismetSystemLibrary.IsValid` _returnvalue) (not (`self.InfiniteAmmo`)))
          (set `local.L_Backpack` _returnvalue)
          ; Check In Backpack
          (bind _outammo (`/Game/Blueprints/Components/AC_Backpack.UpdateAmmoByName` (`local.L_Backpack`) (`self.WeaponName`) (- (`.RoundMax_8_3E092F184B562C4574B110BCF31C5381` (break `/Game/Blueprints/Structures/STRUCT_WeaponStats` (`self.WeaponStats`))) (`self.CurrentRounds`)) false))
          (set `self.CurrentRounds` _outammo)
          (else
            (set `self.CurrentRounds` (`.RoundMax_8_3E092F184B562C4574B110BCF31C5381` (break `/Game/Blueprints/Structures/STRUCT_WeaponStats` (`self.WeaponStats`)))))))
      (:`then_3`
        (if (> (`self.CurrentRounds`) 0)
          (`KismetSystemLibrary.K2_SetTimerDelegate` (`|CreateDelegate` :!event `AfterReloadDelayEnds`) (`.ReloadTime_17_E12FA9884E84FD8781E987B5FF3FFC03` (break `/Game/Blueprints/Structures/STRUCT_WeaponStats` (`self.WeaponStats`))))
          (else
            (`self.UpdateWeaponState` "NewEnumerator4")))))))

(fn `RoundsCount`
  (returns (AllowShooting :type Boolean))
  (bind _result (`/Engine/EditorBlueprintResources/StandardMacros.DecrementInt` (`self.CurrentRounds`))
    (:`  `
      (return (> _result 0)))))

(fn `Shooting`
  (if (`self.ShootInProcess`)
    (if (`|EnumEquality` (`self.CurrentWeaponState`) "NewEnumerator0")
      (`self.SingleShot`)
      (bind _allowshooting (`self.RoundsCount`))
      (if _allowshooting
        (`KismetSystemLibrary.K2_SetTimerDelegate` (`|CreateDelegate` :!event `AfterShotDelayEnds`) (`.ShotTime_15_6532A34E44B712A7BD7D0BAD1F9C405C` (break `/Game/Blueprints/Structures/STRUCT_WeaponStats` (`self.WeaponStats`))))
        (`self.UpdateWeaponState` "NewEnumerator1")
        (else
          (`self.UpdateWeaponState` "NewEnumerator2")
          (if (`self.AutoReload`)
            (`self.Reload`))))
      (else
        (switch `/Game/Blueprints/Enums/ENUM_WeaponState` (`self.CurrentWeaponState`)
          (:`NewEnumerator2`
            _)
          (:`NewEnumerator4`
            _)
          (:`NewEnumerator5`
            _))
        ; flinch feedback
        (if (not (`AudioComponent.IsPlaying` (`self.FlinchAudio`)))
          (`AudioComponent.Play` (`self.FlinchAudio`) 0.0))))))

(fn `ShootInputRecieved`
  (params (InProcess :type Boolean))
  (set `self.ShootInProcess` InProcess))

(fn `ShotFeedback`
  (`AudioComponent.Play` (`self.ShootAudio`) 0.0)
  (bind _returnvalue (`|SpawnActorFromClass` "/Game/Blueprints/Weapon/Projectiles/Effects/BP_MuzzleEffects.BP_MuzzleEffects_C" (`SceneComponent.K2_GetComponentToWorld` (`self.MuzzleScene`)) "Undefined" "MultiplyWithRoot" null null))
  (`self.K2_AttachToComponent` _returnvalue (`self.MuzzleScene`) "None" "SnapToTarget" "SnapToTarget" "KeepRelative" true))

(fn `SingleShot`
  (bind _returnvalue (`|SpawnActorFromClass` (select `/Game/Blueprints/Enums/ENUM_WeaponType` (`.WeaponType_2_BAA875C24868E2297C177092D08B6A91` (break `/Game/Blueprints/Structures/STRUCT_WeaponStats` (`self.WeaponStats`))) :`NewEnumerator0` "/Game/Blueprints/Weapon/Projectiles/BP_Projectile_Pistol.BP_Projectile_Pistol_C" :`NewEnumerator1` "/Game/Blueprints/Weapon/Projectiles/BP_Projectile_Rifle.BP_Projectile_Rifle_C" :`NewEnumerator2` "/Game/Blueprints/Weapon/Projectiles/BP_Projectile_Shotgun.BP_Projectile_Shotgun_C" :`NewEnumerator3` "/Game/Blueprints/Weapon/Projectiles/BP_Projectile_GrenadeLauncher.BP_Projectile_GrenadeLauncher_C" :`NewEnumerator4` "/Game/Blueprints/Weapon/Projectiles/BP_Projectile_SniperRifle.BP_Projectile_SniperRifle_C" :!type "Actor Class Reference") (`SceneComponent.K2_GetComponentToWorld` (`self.MuzzleScene`)) "Undefined" "MultiplyWithRoot" self null))
  (set `self.LastProjectile` _returnvalue)
  (`self.ShotFeedback`))

(fn `UpdateWeaponState`
  (params (CurrentWeaponState :type "/Game/Blueprints/Enums/ENUM_WeaponState Enum" :default "NewEnumerator0"))
  (set `self.CurrentWeaponState` CurrentWeaponState)
  (`self.OnWeaponStatusChanged`)
  (`/Game/Blueprints/GameEntities/BFL_TPAA.PrintStringCustom` (`KismetStringLibrary.Concat_StrStr` "Shooting State is " (`|GetEnumeratorNameAsString` (`self.CurrentWeaponState`))) true (`KismetMathLibrary.SelectColor` (struct :`R` 0.058065 :`G` 1.0 :`A` 1.0) (struct :`R` 0.515625 :`G` 0.000301 :`A` 1.0) (`self.ShootInProcess`)) 1.0))

(fn `UserConstructionScript`
  (`SceneComponent.SetHiddenInGame` (`self.MuzzleArrow`) (not (`self.Debug`)) false))