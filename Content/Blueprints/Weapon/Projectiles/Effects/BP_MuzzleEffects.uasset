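; Muzzle flash effect actor for weapon projectiles, pairing a particle burst with a brief point light flash.
; On BeginPlay it activates the particle system, then plays a timeline at double speed that scales the light's original intensity by its curve.
; Its life span is set to the timeline's scaled length, so the actor removes itself once the flash ends.
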(event `self.ReceiveBeginPlay`
  (`|ExecutionSequence`
    (:`then_0`
      (`ActorComponent.Activate` (`self.ParticleSystem`) true))
    (:`then_1`
      (`TimelineComponent.SetPlayRate` (`self.MuzzleTimeline`) 2.0)
      (set `self.LightIntensity` (`LightComponentBase.Intensity` (`self.PointLight`)))
      (bind (_direction _intense) (`Timeline|MuzzleTimeline`)
        (:`Update`
          (`LightComponent.SetIntensity` (`self.PointLight`) (* _intense (`self.LightIntensity`))))))
    (:`then_2`
      (`self.SetLifeSpan` (`TimelineComponent.GetScaledTimelineLength` (`self.MuzzleTimeline`))))))

(fn `UserConstructionScript`)