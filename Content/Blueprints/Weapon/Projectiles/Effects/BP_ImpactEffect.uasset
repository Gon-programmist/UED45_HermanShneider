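; BP_ImpactEffect is a short-lived projectile impact effect actor that combines surface-specific particles with a light effect.
; On BeginPlay it picks the particle template from the physical material's surface type, with effects only for concrete, wood and flesh (blood).
; A half-rate timeline scales the point light's starting intensity over time.
; The actor's lifespan matches the scaled timeline length, so it removes itself afterward.
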(event `self.ReceiveBeginPlay`
  (`|ExecutionSequence`
    (:`then_0`
      (`ParticleSystemComponent.SetTemplate` (`self.ImpactVFX`) (select `EPhysicalSurface` (`PhysicalMaterial.SurfaceType` (`self.CurrentPhysMat`)) :`SurfaceType1` "/Game/Polygon_BattleRoyale/ParticleFX/FX_Concrete.FX_Concrete" :`SurfaceType2` "/Game/Polygon_BattleRoyale/ParticleFX/FX_Wood.FX_Wood" :`SurfaceType5` "/Game/Polygon_BattleRoyale/ParticleFX/FX_Blood.FX_Blood" :!type "ParticleSystem Object Reference")))
    (:`then_1`
      (`TimelineComponent.SetPlayRate` (`self.ImpactTimeline`) 0.5)
      (set `self.LightIntensity` (`LightComponentBase.Intensity` (`self.PointLight`)))
      (bind (_direction _intense) (`Timeline|ImpactTimeline`)
        (:`Update`
          (`LightComponent.SetIntensity` (`self.PointLight`) (* _intense (`self.LightIntensity`))))))
    (:`then_2`
      (`self.SetLifeSpan` (`TimelineComponent.GetScaledTimelineLength` (`self.ImpactTimeline`))))))

(fn `UserConstructionScript`)