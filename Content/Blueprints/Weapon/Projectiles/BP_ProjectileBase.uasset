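; Base weapon projectile that, on hit, applies physics impulse and damage, spawns impact feedback, then sets its remaining lifespan.
; Collision is briefly disabled at spawn, and hits on the owning weapon or its character are ignored.
; Damage and weapon type come from the owning weapon, with a headshot bone multiplier.
; Non-simulating components get a radial impulse for destructibles; the attached impact effect scales by weapon type and receives the physical material.
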(event `self.ReceiveBeginPlay`
  (`PrimitiveComponent.SetCollisionEnabled` (`self.PtojectileSphere`) "NoCollision")
  (`KismetSystemLibrary.Delay` 0.02)
  (`PrimitiveComponent.SetCollisionEnabled` (`self.PtojectileSphere`) "QueryAndPhysics"))

(event `self.ReceiveHit`
  (params (MyComp :type "PrimitiveComponent Object Reference") (Other :type "Actor Object Reference") (OtherComp :type "PrimitiveComponent Object Reference") (bSelfMoved :type Boolean) (HitLocation :type "Vector Structure") (HitNormal :type "Vector Structure") (NormalImpulse :type "Vector Structure") (Hit :type "HitResult Structure (by ref)"))
  (set `self.CurrentHit` Hit)
  (if (`self.OwnerHitCheck`)
    (`|ExecutionSequence`
      (:`then_0`
        (bind _outweaponstats (message `/Game/Blueprints/GameEntities/BI_Shooting.GetWeaponStats` (`self.GetOwner`)))
        (set `self.CurrentWeaponType` (`.WeaponType_2_BAA875C24868E2297C177092D08B6A91` (break `/Game/Blueprints/Structures/STRUCT_WeaponStats` _outweaponstats))))
      (:`then_1`
        (`self.AddPhysicsImpulse`))
      (:`then_2`
        (`self.ApplyDamageByProjectile`))
      (:`then_3`
        (`self.Feedback`))
      (:`then_4`
        (`self.OnEndOfHit`)))))

(fn `AddPhysicsImpulse`
  (locals (L_OtherComp :type "PrimitiveComponent Object Reference"))
  (bind (_bblockinghit _binitialoverlap _time _distance _location _impactpoint _normal _impactnormal _physmat _hitactor _hitcomponent) (`GameplayStatics.BreakHitResult` (`self.CurrentHit`)))
  (`/Engine/EditorBlueprintResources/StandardMacros.IsValid` _hitcomponent
    (:`Is Valid`
      (set `local.L_OtherComp` _hitcomponent)
      (if (`SceneComponent.IsSimulatingPhysics` (`local.L_OtherComp`) "None")
        (`PrimitiveComponent.AddImpulseAtLocation` (`local.L_OtherComp`) (* (`self.GetVelocity`) (`self.ImpulseMult`)) (`.Location` (`GameplayStatics.BreakHitResult` (`self.CurrentHit`))) "None")
        (else
          ; Only for Destructables
          (`RadialForceComponent.FireImpulse` (`self.RadialForce`)))))))

(fn `ApplyDamageByProjectile`
  (locals (L_Damage :type Integer :default 0))
  (`|ExecutionSequence`
    (:`then_0`
      (bind (_outweaponstats _outcurrentrounds _outcurrentdamage) (message `/Game/Blueprints/GameEntities/BI_Shooting.GetWeaponStats` (`self.GetOwner`)))
      (set `local.L_Damage` _outcurrentdamage))
    (:`then_1`
      (if (== (`.HitBoneName` (`GameplayStatics.BreakHitResult` (`self.CurrentHit`))) "head")
        (set `local.L_Damage` (* (`local.L_Damage`) (`self.HeadshotDamageMult`)))))
    (:`then_2`
      (`GameplayStatics.ApplyDamage` (`.HitActor` (`GameplayStatics.BreakHitResult` (`self.CurrentHit`))) (`KismetMathLibrary.Conv_IntToDouble` (`local.L_Damage`)) null (`self.GetOwner` (`self.GetOwner`)) "/Game/Blueprints/Objects/BP_DamageType.BP_DamageType_C"))))

(fn `Feedback`
  (locals (L_ImpactActor :type "/Game/Blueprints/Weapon/Projectiles/Effects/BP_ImpactEffect Object Reference") (L_Location :type "Vector Structure" :default (0.0 0.0 0.0)) (L_Rotation :type "Rotator Structure" :default (struct)) (L_Scale :type "Vector Structure") (L_PhysMat :type "PhysicalMaterial Object Reference"))
  (bind (_bblockinghit _binitialoverlap _time _distance _location _impactpoint _normal _impactnormal _physmat _hitactor _hitcomponent _hitbonename) (`GameplayStatics.BreakHitResult` (`self.CurrentHit`)))
  (bind (_bblockinghit_2 _binitialoverlap_2 _time_2 _distance_2 _location_2 _impactpoint_2 _normal_2) (`GameplayStatics.BreakHitResult` (`self.CurrentHit`)))
  (bind (_returnvalue_roll _returnvalue_pitch _returnvalue_yaw) (`KismetMathLibrary.BreakRotator` (`KismetMathLibrary.Conv_VectorToRotator` _normal_2)))
  (`|ExecutionSequence`
    (:`then_0`
      (set `local.L_Location` _impactpoint_2)
      (set `local.L_Rotation` (`KismetMathLibrary.MakeRotator` (`KismetMathLibrary.RandomFloatInRange` 0.0 360.0) _returnvalue_pitch _returnvalue_yaw))
      (set `local.L_Scale` (* (1.0 1.0 1.0) (select `/Game/Blueprints/Enums/ENUM_WeaponType` (`self.CurrentWeaponType`) :`NewEnumerator0` 0.75 :`NewEnumerator1` 1.0 :`NewEnumerator2` 0.5 :`NewEnumerator3` 1.0 :`NewEnumerator4` 1.25 :!type "Float (single-precision)")))
      (set `local.L_PhysMat` (`.PhysMat` (`GameplayStatics.BreakHitResult` (`self.CurrentHit`)))))
    (:`then_1`
      (bind _returnvalue (`|SpawnActorFromClass` "/Game/Blueprints/Weapon/Projectiles/Effects/BP_ImpactEffect.BP_ImpactEffect_C" (`KismetMathLibrary.MakeTransform` (`local.L_Location`) (`local.L_Rotation`) (`local.L_Scale`)) "Undefined" "MultiplyWithRoot" null (`local.L_PhysMat`) null))
      (set `local.L_ImpactActor` _returnvalue)
      (`self.K2_AttachToComponent` (`local.L_ImpactActor`) _hitcomponent _hitbonename "KeepWorld" "KeepWorld" "KeepWorld" true))))

(fn `OnEndOfHit`
  (`self.SetLifeSpan` (`self.OnEndOfHitLifespan`)))

(fn `OwnerHitCheck`
  (returns (AbleToHit :type Boolean))
  (bind (_bblockinghit _binitialoverlap _time _distance _location _impactpoint _normal _impactnormal _physmat _hitactor) (`GameplayStatics.BreakHitResult` (`self.CurrentHit`)))
  (return (and (!= _hitactor (`self.GetOwner`)) (!= _hitactor (`self.GetOwner` (`self.GetOwner`))))))

(fn `UserConstructionScript`)