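; Base NPC spawner actor that spawns a set number of BP_NPC instances from a configurable class at its billboard's transform.
; It can begin on BeginPlay, waits an initial delay, then uses a timer between spawns until the count is reached and spawning is flagged as ended.
; Each spawned NPC is stored as the last spawned and receives the spawner's patrolling group when that is non-zero.
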(event `self.ReceiveBeginPlay`
  (if (`self.SpawnOnStart`)
    (`self.BeginSpawn`)))

(event `BeginSpawn`
  (`KismetSystemLibrary.Delay` (`self.PreSpawnDelay`))
  (`self.SpawnOneNPC`))

(fn `EndSpawn`
  (set `self.IsSpawnEnded` true))

(fn `SpawnOneNPC`
  (if (not (`self.IsSpawnEnded`))
    (if (`KismetSystemLibrary.IsValidClass` (`self.SpawnNPCClass`))
      (if (< (`self.Counter`) (`self.NPCsCount`))
        (bind _returnvalue (`|SpawnActorFromClass` (`self.SpawnNPCClass`) (`SceneComponent.K2_GetComponentToWorld` (`self.SpawnPointBillboard`)) "AdjustIfPossibleButAlwaysSpawn" "MultiplyWithRoot" self null))
        (bind _asbp_npc (cast `/Game/Blueprints/Characters/NPC/BP_NPC` _returnvalue))
        (set `self.LastSpawnedNPC` _asbp_npc)
        (`self.UpdatePatrollingGroupForSpawnedNPC`)
        (`/Engine/EditorBlueprintResources/StandardMacros.IncrementInt` (`self.Counter`)
          (:`  `
            (`KismetSystemLibrary.K2_SetTimerDelegate` (`|CreateDelegate` :!event `SpawnOneNPC`) (`self.BetweenSpawnDelay`))))
        (else
          (`self.EndSpawn`))))))

(fn `UpdatePatrollingGroupForSpawnedNPC`
  (if (!= (`self.PatrollingGroup`) 0)
    (`/Game/Blueprints/Characters/NPC/BP_NPC.UpdatePatrollingGroup` (`self.LastSpawnedNPC`) (`self.PatrollingGroup`))))

(fn `UserConstructionScript`)