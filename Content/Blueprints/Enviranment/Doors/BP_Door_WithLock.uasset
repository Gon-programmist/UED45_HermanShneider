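; Lockable child door Blueprint that stays closed until the interacting actor's backpack holds all needed quest keys.
; While locked, interaction plays a timeline wiggle and checks the AC_Backpack; unlocked, it uses parent door behavior.
; Unlocking swaps the lock icon to open, hides it after a delay, and writes door status to the save game.
; Save overrides skip parent logic, persisting and restoring the unlock instead of the open state.
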(event `self.ReceiveBeginPlay`
  (`parent.ReceiveBeginPlay`))

(event `TryOpenLockedDoor`
  (bind (_direction _dooranglemult) (`Timeline|LockedFeedbackTimeline` :!via `PlayFromStart`)
    (:`Update`
      (`SceneComponent.K2_SetRelativeRotation` (`self.DoorScene`) (`KismetMathLibrary.MakeRotator` 0.0 0.0 (* (`self.LockedDoorAngle`) _dooranglemult (`self.CurrentDotProduct`))) false false))))

(event `UnlockFeedback`
  (`StaticMeshComponent.SetStaticMesh` (`self.IconLockClosedMesh`) "/Game/Polygon_Prototype/Meshes/Icons/SM_Icon_Lock_Open_01.SM_Icon_Lock_Open_01")
  (`KismetSystemLibrary.Delay` 2.0)
  (`SceneComponent.SetVisibility` (`self.IconLockClosedMesh`) false false))

(fn `CheckKeysInBackpack`
  (locals (L_Backpack :type "/Game/Blueprints/Components/AC_Backpack Object Reference") (L_ItemName :type Name))
  (bind _returnvalue (`self.GetComponentByClass` (`self.ActorOfInteraction`) "/Game/Blueprints/Components/AC_Backpack.AC_Backpack_C"))
  (if (`KismetArrayLibrary.Array_IsValidIndex` (`self.NededKeys`))
    (`/Engine/EditorBlueprintResources/StandardMacros.IsValid` _returnvalue
      (:`Is Valid`
        (set `local.L_Backpack` _returnvalue)
        (for _array_element (`self.NededKeys`)
          (set `local.L_ItemName` _array_element)
          (bind _success (`/Game/Blueprints/Components/AC_Backpack.CheckQuestItem` (`local.L_Backpack`) (`local.L_ItemName`)))
          (if _success
            (`KismetArrayLibrary.Array_AddUnique` (`self.CheckKeys`) (`local.L_ItemName`))))
        (if (`KismetArrayLibrary.Array_Identical` (`self.NededKeys`) (`self.CheckKeys`))
          (`self.UnlockDoor`)
          (else
            (`KismetArrayLibrary.Array_Clear` (`self.CheckKeys`))))))))

(fn `ConfigureOpenDoorOnConstruct`
  (if (`self.bIsDoorLocked`)
    (set `self.bIsDoorOpen` (not (`self.bIsDoorLocked`))))
  (`parent.ConfigureOpenDoorOnConstruct`))

(fn `SaveOpenDoorStatus`)

(fn `UnlockDoor`
  (set `self.bIsDoorLocked` false)
  (`|ExecutionSequence`
    (:`then_0`
      (`self.UnlockFeedback`))
    (:`then_1`
      (bind _outsavegameobj (`/Game/Blueprints/GameEntities/BML_TPAA.SimpleSaveGameCheck`)
        (:`IsValid`
          (`BlueprintMapLibrary.Map_Add` (`/Game/Blueprints/Objects/BP_SaveGameObject.DoorStatus` _outsavegameobj) (`/Game/Blueprints/GameEntities/BFL_TPAA.GetObjectIndexForSaveData` self) (not (`self.bIsDoorLocked`))))))))

(fn `UpdateDoorOpenOnSaveData`
  (if (`self.IsItSaved`)
    (if (`self.IsItUsed`)
      (`KismetArrayLibrary.Array_Clear` (`self.CheckKeys`))
      (`self.UnlockDoor`))))

(fn `UpdateDoorVisual`
  (if (not (`self.bIsDoorLocked`))
    (`parent.UpdateDoorVisual`)
    (else
      (`|ExecutionSequence`
        (:`then_0`
          (`self.TryOpenLockedDoor`))
        (:`then_1`
          (`self.CheckKeysInBackpack`))))))

(fn `UserConstructionScript`
  (`parent.UserConstructionScript`)
  (`SceneComponent.SetVisibility` (`self.IconLockClosedMesh`) (`self.bIsDoorLocked`) false))