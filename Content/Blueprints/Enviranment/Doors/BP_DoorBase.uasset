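; Base interactable door actor that swings open or closed on a timeline and persists its open state in the save game.
; Interact uses a dot product between the Arrow and the interacting actor to pick swing direction, remembering it for closing.
; The timeline rotates DoorScene yaw, with mesh collision disabled during motion, and saves the state when finished.
; BeginPlay restores saved state; the construction script previews it and sizes the collision box.
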(event `self.ReceiveBeginPlay`
  (`self.ConfigureDoor`))

(event `OpenDoor`
  (if (not (`self.bInProgress`))
    (if (not (`self.bIsDoorOpen`))
      (`self.UpdateInProgress` true)
      (bind (_direction _dooropenprogress) (`Timeline|DoorProgressTimeline` :!via `PlayFromStart` :!label _label)
        (:`Update`
          (`SceneComponent.K2_SetRelativeRotation` (`self.DoorScene`) (`KismetMathLibrary.MakeRotator` 0.0 0.0 (* (`self.MaxDoorOpenAngle`) _dooropenprogress (`KismetMathLibrary.SelectFloat` (`self.PreviusDotProduct`) (`self.CurrentDotProduct`) (`self.bIsDoorOpen`)))) false false))
        (:`Finished`
          (`|ExecutionSequence`
            (:`then_0`
              (set `self.PreviusDotProduct` (`self.CurrentDotProduct`))
              (`self.UpdateInProgress` false)
              (switch `ETimelineDirection` _direction
                (:`Forward`
                  (set `self.bIsDoorOpen` true))
                (:`Backward`
                  (set `self.bIsDoorOpen` false))))
            (:`then_1`
              (`self.SaveOpenDoorStatus`))))))))

(event `CloseDoor`
  (if (not (`self.bInProgress`))
    (if (`self.bIsDoorOpen`)
      (`self.UpdateInProgress` true)
      (goto _label :!via `ReverseFromEnd`))))

(fn `ConfigureDoor`
  (`|ExecutionSequence`
    (:`then_0`
      (`TimelineComponent.SetPlayRate` (`self.DoorProgressTimeline`) (`self.DoorOpenSpeed`)))
    (:`then_1`
      (`self.ConfigureSavedDoor`)
      (`self.UpdateDoorOpenOnSaveData`))))

(fn `ConfigureOpenDoorOnConstruct`
  (`SceneComponent.K2_SetRelativeRotation` (`self.DoorScene`) (`KismetMathLibrary.MakeRotator` 0.0 0.0 (`KismetMathLibrary.SelectFloat` (`self.MaxDoorOpenAngle`) 0.0 (`self.bIsDoorOpen`))) false false))

(fn `ConfigureSavedDoor`
  (bind _outsavegameobj (`/Game/Blueprints/GameEntities/BML_TPAA.SimpleSaveGameCheck`)
    (:`IsValid`
      (bind (_value _returnvalue) (`BlueprintMapLibrary.Map_Find` (`/Game/Blueprints/Objects/BP_SaveGameObject.DoorStatus` _outsavegameobj) (`/Game/Blueprints/GameEntities/BFL_TPAA.GetObjectIndexForSaveData` self)))
      (if _returnvalue
        (set `self.IsItSaved` _returnvalue)
        (set `self.IsItUsed` _value)))))

(fn `Interact`
  (params (InteractActor :type "Actor Object Reference"))
  (returns (Succes :type Boolean))
  (set `self.ActorOfInteraction` InteractActor)
  (set `self.CurrentDotProduct` (`KismetMathLibrary.SelectFloat` 1.0 -1.0 (> (`/Game/Blueprints/GameEntities/BFL_TPAA.DotProductOfTwoComponents` (`self.Arrow`) (`Actor.RootComponent` (`self.ActorOfInteraction`))) 0.0)))
  (`self.UpdateDoorVisual`)
  (return true))

(fn `SaveOpenDoorStatus`
  (bind _outsavegameobj (`/Game/Blueprints/GameEntities/BML_TPAA.SimpleSaveGameCheck`)
    (:`IsValid`
      (`BlueprintMapLibrary.Map_Add` (`/Game/Blueprints/Objects/BP_SaveGameObject.DoorStatus` _outsavegameobj) (`/Game/Blueprints/GameEntities/BFL_TPAA.GetObjectIndexForSaveData` self) (`self.bIsDoorOpen`)))))

(fn `SwitchDoorOpen`
  (set `self.bIsDoorOpen` (not (`self.bIsDoorOpen`))))

(fn `UpdateBoxExtent`
  (bind (_doorboxcollisionextent_x _doorboxcollisionextent_y _doorboxcollisionextent_z) (`KismetMathLibrary.BreakVector` (`self.DoorBoxCollisionExtent`)))
  ; Locations update construction
  (`BoxComponent.SetBoxExtent` (`self.DoorBoxCollison`) (`self.DoorBoxCollisionExtent`) true)
  (`SceneComponent.K2_SetRelativeLocation` (`self.DoorBoxCollison`) (`KismetMathLibrary.MakeVector` 0.0 0.0 _doorboxcollisionextent_z) false false))

(fn `UpdateDoorOpenOnSaveData`
  (set `self.bIsDoorOpen` (`self.IsItUsed`))
  (`self.ConfigureOpenDoorOnConstruct`))

(fn `UpdateDoorVisual`
  (if (`self.bIsDoorOpen`)
    (`self.CloseDoor`)
    (else
      (`self.OpenDoor`))))

(fn `UpdateInProgress`
  (params (bInProgress :type Boolean))
  (set `self.bInProgress` bInProgress)
  (`PrimitiveComponent.SetCollisionEnabled` (`self.DoorMesh`) (select `bool` (`self.bInProgress`) :`false` "QueryAndPhysics" :`true` "NoCollision" :!type "ECollisionEnabled Enum")))

(fn `UserConstructionScript`
  (`|ExecutionSequence`
    (:`then_0`
      (`self.ConfigureOpenDoorOnConstruct`))
    (:`then_1`
      (`self.UpdateBoxExtent`))))