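; Patrol waypoint actor placed in a level to mark a numbered point within an NPC patrol group.
; The construction script labels it with its group and point number, or a prompt to set the group if it is zero.
; Overlap events track BP_NPC actors on the point and keep a Vacant flag that is true only when none remain.
; The arrow, mesh and text stay hidden in game unless Debug is set.
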(event `self.ReceiveBeginPlay`
  (`SceneComponent.SetHiddenInGame` (`self.Arrow`) (not (`self.Debug`)) false)
  (`SceneComponent.SetHiddenInGame` (`self.StaticMesh`) (not (`self.Debug`)) false)
  (`SceneComponent.SetHiddenInGame` (`self.TextRender`) (not (`self.Debug`)) false))

(event `self.ReceiveActorBeginOverlap`
  (params (OtherActor :type "Actor Object Reference"))
  (set `self.OverlappedActor` OtherActor)
  (cast `/Game/Blueprints/Characters/NPC/BP_NPC` (`self.OverlappedActor`))
  (`KismetArrayLibrary.Array_AddUnique` (`self.OverlappedActors`) (`self.OverlappedActor`))
  (set `self.Vacant` false))

(event `self.ReceiveActorEndOverlap`
  (params (OtherActor :type "Actor Object Reference"))
  (set `self.ActorEndOverlapped` OtherActor)
  (cast `/Game/Blueprints/Characters/NPC/BP_NPC` (`self.ActorEndOverlapped`))
  (`KismetArrayLibrary.Array_RemoveItem` (`self.OverlappedActors`) (`self.ActorEndOverlapped`))
  (set `self.Vacant` (`KismetArrayLibrary.Array_IsEmpty` (`self.OverlappedActors`))))

(fn `UserConstructionScript`
  (if (!= (`self.PatrolGroup`) 0)
    (`TextRenderComponent.K2_SetText` (`self.TextRender`) (`|FormatText` "Group{A} \nPoint{B}" (`self.PatrolGroup`) (`self.PatrolPointNumber`)))
    (else
      (`TextRenderComponent.K2_SetText` (`self.TextRender`) (`|FormatText` "SetPatrolGroup")))))