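; Base shooting target actor that shows its health on a text label and gets knocked loose when killed.
; Health component updates switch the label between current/max HP and a death message.
; On death, the target mesh simulates physics with a small random impulse and the actor expires after a short lifespan.
; It also reports its Name and the main stats struct looked up by that name.
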(event `self.AC_Health.OnHealthUpdated`
  (params (CurrentHP :type Integer) (IsDead :type Boolean) (IsItDamage :type Boolean))
  (`TextRenderComponent.K2_SetText` (`self.TextRender`) (select `bool` IsDead :`false` (`|FormatText` "HP {hp}/{MaxHP} " (`/Game/Blueprints/Components/AC_Health.CurrentHP` (`self.AC_Health`)) (`/Game/Blueprints/Components/AC_Health.MaxHP` (`self.AC_Health`))) :`true` (`|FormatText` "{A} IS DEAD!" (`KismetSystemLibrary.GetDisplayName` self)))))

(event `self.AC_Health.OnDied`
  (`PrimitiveComponent.SetSimulatePhysics` (`self.TargetMesh`) true)
  (`PrimitiveComponent.AddImpulse` (`self.TargetMesh`) (`KismetMathLibrary.MakeVector` (`KismetMathLibrary.RandomFloatInRange` -100.0 100.0) (`KismetMathLibrary.RandomFloatInRange` -100.0 100.0) (`KismetMathLibrary.RandomFloatInRange` -100.0 100.0)) "None" false)
  (`self.SetLifeSpan` 5.0))

(fn `GetCurrentCharName`
  (returns (Success :type Boolean) (CurrentCharName :type Name))
  (return true (`self.Name`)))

(fn `GetMainStatsStruct`
  (returns (Success :type Boolean) (MainStats :type "/Game/Blueprints/Structures/STRUCT_MainStats Structure"))
  (bind (_success _mainstats) (`/Game/Blueprints/GameEntities/BFL_TPAA.GetMainStatsStructByName` (`self.Name`)))
  (return _success _mainstats))

(fn `UserConstructionScript`)