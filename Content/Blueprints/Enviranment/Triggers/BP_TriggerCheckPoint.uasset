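; Checkpoint trigger that saves the game when an actor with a camera component, likely the player, overlaps it.
; The overlap fires once and, if the trigger is unused, marks its save-data index true in the save game's TriggerStatus map.
; It then asks the game instance to save and destroys itself.
; The construction script sets trigger mesh visibility from a variable.
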(event `self.ReceiveBeginPlay`
  (`parent.ReceiveBeginPlay`))

(event `self.ReceiveActorBeginOverlap`
  (params (OtherActor :type "Actor Object Reference"))
  (`parent.ReceiveActorBeginOverlap` OtherActor)
  (`/Engine/EditorBlueprintResources/StandardMacros.IsValid` (`self.GetComponentByClass` (`self.OverlappedActor`) "/Script/Engine.CameraComponent")
    (:`Is Valid`
      (`/Engine/EditorBlueprintResources/StandardMacros.DoOnce` false
        (:`Completed`
          (if (not (`self.IsItUsed`))
            (`|ExecutionSequence`
              (:`then_0`
                (bind _outsavegameobj (`/Game/Blueprints/GameEntities/BML_TPAA.SimpleSaveGameCheck`)
                  (:`IsValid`
                    (`BlueprintMapLibrary.Map_Add` (`/Game/Blueprints/Objects/BP_SaveGameObject.TriggerStatus` _outsavegameobj) (`/Game/Blueprints/GameEntities/BFL_TPAA.GetObjectIndexForSaveData` self) true))))
              (:`then_1`
                (message `/Game/Blueprints/GameEntities/BI_SaveGame.SaveGameData` (`GameplayStatics.GetGameInstance`) ""))
              (:`then_2`
                (`self.K2_DestroyActor`)))))))))

(fn `UserConstructionScript`
  (`parent.UserConstructionScript`)
  (`SceneComponent.SetVisibility` (`self.SceneMeshes`) (`self.TriggerMeshesVisibility`) true))