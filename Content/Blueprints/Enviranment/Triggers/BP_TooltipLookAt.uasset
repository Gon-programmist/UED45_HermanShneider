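; BP_TooltipLookAt is a tooltip trigger actor that keeps its Arrow component facing the camera of the overlapped actor.
; Every tick it calls LookingAtPlayerCamera, which checks that OverlappedActor and its CameraComponent are valid.
; It then sets the Arrow's world rotation with FindLookAtRotation toward that camera.
; Tick and construction also run the parent logic, and no graph here assigns OverlappedActor.
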(event `self.ReceiveTick`
  (params (DeltaSeconds :type "Float (single-precision)"))
  (`parent.ReceiveTick` DeltaSeconds)
  (`self.LookingAtPlayerCamera`))

(fn `LookingAtPlayerCamera`
  (bind _overlappedactor (`self.OverlappedActor`)
    (:`then`
      (bind _returnvalue (`self.GetComponentByClass` _overlappedactor "/Script/Engine.CameraComponent"))
      (`/Engine/EditorBlueprintResources/StandardMacros.IsValid` _returnvalue
        (:`Is Valid`
          (`SceneComponent.K2_SetWorldRotation` (`self.Arrow`) (`KismetMathLibrary.FindLookAtRotation` (`SceneComponent.K2_GetComponentLocation` (`self.Arrow`)) (`SceneComponent.K2_GetComponentLocation` _returnvalue)) false false))))
    (:`else`)))

(fn `UserConstructionScript`
  (`parent.UserConstructionScript`))