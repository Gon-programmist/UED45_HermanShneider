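; BP_Trigger_Sound is a trigger actor that plays a configurable sound while something overlaps it.
; BeginPlay assigns the Sound and UI-sound flag to its Audio component.
; Begin overlap starts playback unless already playing, and end overlap fades out over one second with a matching delayed stop, without filtering the overlapping actor.
; The construction script labels a TextRender component with the assigned sound's name.
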(event `self.ReceiveBeginPlay`
  (`parent.ReceiveBeginPlay`)
  (`AudioComponent.SetSound` (`self.Audio`) (`self.Sound`))
  (`AudioComponent.SetUISound` (`self.Audio`) (`self.In UISound`)))

(event `self.ReceiveActorBeginOverlap`
  (params (OtherActor :type "Actor Object Reference"))
  (`parent.ReceiveActorBeginOverlap` OtherActor)
  (if (not (`AudioComponent.IsPlaying` (`self.Audio`)))
    (`AudioComponent.Play` (`self.Audio`) 0.0)))

(event `self.ReceiveActorEndOverlap`
  (params (OtherActor :type "Actor Object Reference"))
  (`parent.ReceiveActorEndOverlap` OtherActor)
  (`AudioComponent.FadeOut` (`self.Audio`) 1.0 0.0 "SCurve")
  (`AudioComponent.StopDelayed` (`self.Audio`) 1.0))

(fn `UserConstructionScript`
  (`parent.UserConstructionScript`)
  (`self.Sound`
    (:`then`
      (`TextRenderComponent.K2_SetText` (`self.TextRender`) (`|FormatText` "Audio:  \n{Cue}" (`KismetSystemLibrary.GetDisplayName` (`self.Sound`)))))
    (:`else`)))