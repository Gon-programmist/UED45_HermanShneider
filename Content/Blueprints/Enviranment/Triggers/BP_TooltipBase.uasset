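; Base trigger actor for in-world tooltips that show a text render while an actor overlaps it.
; The construction script sizes the box from BoxExtent, raises it by its Z extent, moves the arrow to TextLocation and applies the configured text.
; Text starts hidden on BeginPlay, and any begin or end overlap toggles it without filtering the actor, storing or clearing OverlappedActor.
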(event `self.ReceiveBeginPlay`
  (`self.UpdateTextVisibility` false))

(event `self.ReceiveActorBeginOverlap`
  (params (OtherActor :type "Actor Object Reference"))
  (set `self.OverlappedActor` OtherActor)
  (`self.UpdateTextVisibility` true))

(event `self.ReceiveActorEndOverlap`
  (params (OtherActor :type "Actor Object Reference"))
  (set `self.OverlappedActor` null)
  (`self.UpdateTextVisibility` false))

(fn `UpdateTextVisibility`
  (params (InVisibility :type Boolean :default true))
  (`SceneComponent.SetVisibility` (`self.TextRender`) InVisibility false))

(fn `UserConstructionScript`
  (bind (_boxextent_x _boxextent_y _boxextent_z) (`KismetMathLibrary.BreakVector` (`self.BoxExtent`)))
  (`|ExecutionSequence`
    (:`then_0`
      ; Locations update construction
      (`BoxComponent.SetBoxExtent` (`self.Box`) (`self.BoxExtent`) true)
      (`SceneComponent.K2_SetRelativeLocation` (`self.Box`) (`KismetMathLibrary.MakeVector` 0.0 0.0 _boxextent_z) false false)
      (`SceneComponent.K2_SetRelativeLocation` (`self.Arrow`) (`self.TextLocation`) false false))
    (:`then_1`
      (`TextRenderComponent.K2_SetText` (`self.TextRender`) (`self.Text`)))))