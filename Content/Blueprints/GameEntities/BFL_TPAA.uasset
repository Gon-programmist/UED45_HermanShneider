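; BFL_TPAA is a Blueprint function library of shared helpers for stats lookup, save data keys and debugging.
; It fetches main and weapon stats rows by name from DT_AllStats and DT_WeaponStats, returning a success flag and printing on failure.
; It also builds save-data Names from level and object display names, wraps PrintString, and computes a facing dot product between two scene components while drawing debug arrows.
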(fn `DotProductOfTwoComponents`
  (params (InSceneComponentFromDotProduct :type "SceneComponent Object Reference") (InSceneComponentToDotProduct :type "SceneComponent Object Reference"))
  (returns (OutDotProductResult :type "Float (double-precision)"))
  (bind _inscenecomponentfromdotproduct (`local.InSceneComponentFromDotProduct`))
  (bind _returnvalue (`SceneComponent.K2_GetComponentLocation` _inscenecomponentfromdotproduct))
  (`|ExecutionSequence`
    (:`then_0`
      (`KismetSystemLibrary.DrawDebugArrow` null (`SceneComponent.K2_GetComponentLocation` (`local.InSceneComponentFromDotProduct`)) (`SceneComponent.K2_GetComponentLocation` (`local.InSceneComponentToDotProduct`)) 15.0 (struct :`R` 0.04122 :`G` 0.051854 :`B` 0.15625 :`A` 1.0) 3.0 4.0)
      (`KismetSystemLibrary.DrawDebugArrow` null _returnvalue (+ _returnvalue (* (`SceneComponent.GetForwardVector` _inscenecomponentfromdotproduct) 100.0)) 15.0 (struct :`R` 0.428691 :`B` 1.0 :`A` 1.0) 3.0 4.0))
    (:`then_1`
      (return (`KismetMathLibrary.Dot_VectorVector` (`KismetMathLibrary.Normal` (- (`SceneComponent.K2_GetComponentLocation` (`local.InSceneComponentToDotProduct`)) (`SceneComponent.K2_GetComponentLocation` (`local.InSceneComponentFromDotProduct`)))) (`SceneComponent.GetForwardVector` (`local.InSceneComponentFromDotProduct`)))))))

(fn `GetMainStatsStructByName`
  (params (InName :type Name))
  (returns (Success :type Boolean) (MainStats :type "/Game/Blueprints/Structures/STRUCT_MainStats Structure"))
  (bind _returnvalue (`|GetDataTableRow` "/Game/Blueprints/DataTables/DT_AllStats.DT_AllStats" InName)
    (:`then`
      (return true _returnvalue))
    (:`RowNotFound`
      (`KismetSystemLibrary.PrintString` null "Configure Stats Failed: Current Name not found in DT" false)
      (return false))))

(fn `GetObjectIndexForSaveData`
  (params (InObj :type "Object Object Reference"))
  (returns (OutSaveIndex :type Name))
  (bind _returnvalue (`GameplayStatics.GetCurrentLevelName` (`local.InObj`)))
  (return (`KismetStringLibrary.Conv_StringToName` (`KismetStringLibrary.Concat_StrStr` _returnvalue "_" (`KismetSystemLibrary.GetDisplayName` (`local.InObj`))))))

(fn `GetWeaponStatsStructByName`
  (params (InWeaponName :type Name))
  (returns (Success :type Boolean) (OutWeaponStats :type "/Game/Blueprints/Structures/STRUCT_WeaponStats Structure"))
  (bind _returnvalue (`|GetDataTableRow` "/Game/Blueprints/DataTables/DT_WeaponStats.DT_WeaponStats" InWeaponName)
    (:`then`
      (return true _returnvalue))
    (:`RowNotFound`
      (`KismetSystemLibrary.PrintString` null "Configure Stats Failed: Current Name not found in DT" false)
      (return false))))

(fn `PrintStringCustom`
  (params (InString :type String) (bPrintToScreen :type Boolean) (TextColor :type "LinearColor Structure") (Duration :type "Float (single-precision)") (Key :type Name))
  (`KismetSystemLibrary.PrintString` null InString bPrintToScreen true TextColor Duration Key))